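; BP_FinalDoor is a locked double dungeon door that opens only once it has been given a key.
; The HasKey event sets the Key flag, which Interaction checks before playing a Timeline.
; The Timeline swings the right and left leaves 90 degrees in opposite yaw directions.
; An event track on that Timeline plays the door sound at world origin rather than at the door.
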(event Custom|HasKey
  (Variables|Default|SetKey true))

(event EventBeginPlay)

(event Collision|EventActorBeginOverlap
  (params (OtherActor :type Actor%20Object%20Reference)))

(event EventTick
  (params (DeltaSeconds :type Float%20%28single-precision%29)))

(event EventInteraction
  (if (Variables|Default|GetKey)
    (bind _newtrack_0 (Timeline|Timeline Play)
      (:Update
        (Transformation|SetRelativeRotation (Variables|Default|GetSM_DoorWay_Large_Door_Right) (Math|Rotator|MakeRotator 0.0 0.0 (Math|Float|Lerp 0.0 9e+01 _newtrack_0)) false false)
        (Transformation|SetRelativeRotation (Variables|Default|GetSM_DoorWay_Large_Door_Left) (Math|Rotator|MakeRotator 0.0 0.0 (* (Math|Float|Lerp 0.0 9e+01 _newtrack_0) -1.0)) false false))
      (:NewTrack_1
        (Audio|PlaySoundatLocation "/Game/Audio/Sfx/Sfx_Door_Dungeon.Sfx_Door_Dungeon" "0, 0, 0" "0, 0, 0" 1.0 1.0 0.0 0 0 0 0)))))

(fn ConstructionScript)